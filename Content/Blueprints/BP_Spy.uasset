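; BP_Spy is an AI-moved pawn that patrols back and forth along the world X axis.
; BeginPlay starts it moving left, toward negative X, despite a comment saying right.
; Left and right events each issue an AIMoveTo a short step from the current nav agent location.
; Success repeats the same direction and failure switches to the other, so the spy reverses whenever a move fails.
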(event `Spy_Right`
  ; Moves The Spy Right
  (`|AIMoveTo` self (+ (`self.GetNavAgentLocation`) (50.0 0.0 0.0)) null 10.0
    (:`OnSuccess`
      ; If Movement fails, do Spy Left Event
      (`self.Spy_Right`))
    (:`OnFail`
      (`self.Spy_Left`))))

(event `Spy_Left`
  ; Sames As Above but Moves The Spy Left
  (`|AIMoveTo` self (+ (`self.GetNavAgentLocation`) (-50.0 0.0 0.0)) null 10.0
    (:`OnSuccess`
      (`self.Spy_Left`))
    (:`OnFail`
      (`self.Spy_Right`))))

(event `self.ReceiveBeginPlay`
  ; Starts The Spy Running Right
  (`self.Spy_Left`))

(fn `UserConstructionScript`)